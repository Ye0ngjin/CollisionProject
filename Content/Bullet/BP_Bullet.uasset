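; BP_Bullet is a physics-driven projectile that knocks characters into ragdoll.
; On BeginPlay its Sphere component gets a forward impulse and a timer starts, which calls LifeTime to destroy the actor after a few seconds.
; When the Sphere hits a ThirdPersonCharacter, it calls DoRagdoll on it and pushes its mesh with the amplified hit normal impulse.
; The bullet is not destroyed on impact, only by the timer.
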(event OnComponentHit(Sphere)
  (params (HitComponent :type Primitive%20Component%20Object%20Reference) (OtherActor :type Actor%20Object%20Reference) (OtherComp :type Primitive%20Component%20Object%20Reference) (NormalImpulse :type Vector :default "0, 0, 0") (Hit :type Hit%20Result%20Structure%20%28by%20ref%29))
  (bind _asthird_person_character (Utilities|Casting|CastToThirdPersonCharacter OtherActor))
  (Default|DoRagdoll _asthird_person_character)
  (Physics|AddImpulse (Variables|/Script/Engine.Character|GetMesh _asthird_person_character) (* NormalImpulse 1e+01) "None" false))

(event EventBeginPlay
  (Physics|AddImpulse (Variables|Default|GetSphere) (* (Math|Vector|GetForwardVector (Variables|Default|GetSphere)) 5e+03) "None" false)
  (Utilities|Time|SetTimerbyFunctionName 0 "LifeTime" 5.0))

(event Collision|EventActorBeginOverlap
  (params (OtherActor :type Actor%20Object%20Reference)))

(event EventTick
  (params (DeltaSeconds :type Float%20%28single-precision%29)))

(fn ConstructionScript)

(fn LifeTime
  (Actor|DestroyActor))